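; BP_Interactable is an interactable actor that changes its Cube's color while it has focus.
; On BeginPlay it creates a dynamic material instance on the Cube and caches its Color parameter as the default.
; StartFocus sets Color to FocusedColor, and EndFocus restores the cached default.
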(event `self.ReceiveBeginPlay`
  (bind _returnvalue (`PrimitiveComponent.CreateDynamicMaterialInstance` (`self.Cube`) 0 null "None"))
  (bind _output_get (set `self.MaterialInst` _returnvalue))
  (bind _returnvalue_2 (`MaterialInstanceDynamic.K2_GetVectorParameterValue` _output_get "Color"))
  (set `self.DefaultColor` _returnvalue_2))

(event `InteractInterface.StartFocus`
  (`MaterialInstanceDynamic.SetVectorParameterValue` (`self.MaterialInst`) "Color" (`self.FocusedColor`)))

(event `InteractInterface.EndFocus`
  (`MaterialInstanceDynamic.SetVectorParameterValue` (`self.MaterialInst`) "Color" (`self.DefaultColor`)))

(fn `UserConstructionScript`)