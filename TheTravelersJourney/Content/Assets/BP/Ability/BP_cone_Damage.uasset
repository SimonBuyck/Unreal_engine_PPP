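; BP_cone_Damage is a short-lived cone damage area for an ability, oriented to the player's rotation when it begins play.
; A looping one-second timer applies Damage to every actor overlapping the Cone, excluding the player character.
; Each tick decrements Delay, which acts as the remaining pulse count, and the actor destroys itself on the tick after it reaches zero.
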(event `self.ReceiveBeginPlay`
  (bind _asmy_character_ (cast `/Game/MyCharacter_` (`GameplayStatics.GetPlayerPawn` 0)))
  (`self.K2_SetActorRotation` (`self.K2_GetActorRotation` _asmy_character_))
  (`KismetSystemLibrary.K2_SetTimerDelegate` (delegate `CustomEvent_0`) 1.0 true))

(event `CustomEvent_0`
  (if (<= (`self.delay`) 0)
    (`self.K2_DestroyActor`)
    (else
      (for _array_element (`PrimitiveComponent.GetOverlappingActors` (`self.Cone`) null)
        (bind _asmy_character_ (cast `/Game/MyCharacter_` (`GameplayStatics.GetPlayerPawn` 0)))
        (if (not (== _asmy_character_ _array_element))
          (`GameplayStatics.ApplyDamage` _array_element (`KismetMathLibrary.Conv_IntToDouble` (`self.damage`)))))
      (set `self.delay` (- (`self.delay`) 1)))))

(fn `UserConstructionScript`)